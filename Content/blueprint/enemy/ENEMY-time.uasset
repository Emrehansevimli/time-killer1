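; Enemy character that chases the player, costing health and time on contact and awarding score when killed.
; An AI MoveTo targets the player, retrying on failure; on arrival it applies damage, subtracts from the player's Time and destroys itself.
; Damage reduces Can; at exactly zero it plays a Beholder death animation, stops movement, adds score, then after a delay destroys itself and spawns a Time10 actor.
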(event Custom|move%20towerd%20player
  (bind _asbp_first_person_character (Utilities|Casting|CastToBP_FirstPersonCharacter (Game|GetPlayerCharacter 0)))
  (bind _output_get (Variables|Default|Setkarakter%20ref _asbp_first_person_character))
  (CallFunction|Rotation)
  (AI|AIMoveTo self (Variables|Default|Getplayer%20pos) _output_get 5.0 false
    (:OnSuccess
      (CallFunction|KilPlayer)
      (Actor|DestroyActor))
    (:OnFail
      (CallFunction|MoveTowerdPlayer))))

(event Custom|gt%20player%20position
  (Variables|Default|Setplayer%20pos (Transformation|GetActorLocation (Variables|Default|Getkarakter%20ref))))

(event Custom|kil%20player
  (bind _asbp_first_person_character (Utilities|Casting|CastToBP_FirstPersonCharacter (Game|GetPlayerCharacter 0)))
  (if (not (Variables|Default|Getcan0mı))
    (Game|Damage|ApplyDamage _asbp_first_person_character 5.0 0 0)
    (Variables|/Game/FirstPerson/Blueprints/BP_FirstPersonCharacter.BP_FirstPersonCharacter_C|Settime _asbp_first_person_character (- (Variables|/Game/FirstPerson/Blueprints/BP_FirstPersonCharacter.BP_FirstPersonCharacter_C|Gettime _asbp_first_person_character) 5.0))))

(event Custom|rotation
  (Variables|Default|Setplayer%20rotation (Math|Rotator|GetRotationXVector (Transformation|GetActorRotation (Variables|Default|Getkarakter%20ref)))))

(event EventBeginPlay
  (CallFunction|MoveTowerdPlayer))

(event EventTick
  (params (DeltaSeconds :type Float%20%28single-precision%29))
  (CallFunction|GtPlayerPosition))

(event Game|Damage|EventAnyDamage
  (params (Damage :type Float%20%28single-precision%29) (DamageType :type Damage%20Type%20Object%20Reference) (InstigatedBy :type Controller%20Object%20Reference) (DamageCauser :type Actor%20Object%20Reference))
  (bind _karakter_ref (Variables|Default|Getkarakter%20ref))
  (bind _output_get (Variables|Default|Setcan (- (Variables|Default|Getcan) Damage)))
  (if (== _output_get 0.0)
    (Variables|Default|Setcan0mı true)
    (Components|Animation|PlayAnimation (Variables|Character|GetMesh) "/Game/blueprint/enemy/Beholder_Die_ANIM1.Beholder_Die_ANIM1" false)
    (Pawn|Components|CharacterMovement|DisableMovement (Variables|Character|GetCharacterMovement))
    (Variables|/Game/FirstPerson/Blueprints/BP_FirstPersonCharacter.BP_FirstPersonCharacter_C|Setscore _karakter_ref (+ (Variables|/Game/FirstPerson/Blueprints/BP_FirstPersonCharacter.BP_FirstPersonCharacter_C|Getscore _karakter_ref) 5))
    (Utilities|FlowControl|Delay 1.0)
    (Actor|DestroyActor)
    (Game|SpawnActorfromClass "/Game/blueprint/time-10.time-10_C" (Math|Transform|MakeTransform (Transformation|GetActorLocation) "0, 0, 0" "1.000000,1.000000,1.000000") "Undefined" "MultiplyWithRoot" 0 0)))

(fn ConstructionScript)