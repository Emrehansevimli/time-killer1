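; Enemy spawner Blueprint that periodically spawns enemies at random points across a fixed world area.
; BeginPlay starts a looping timer on the spawn event at the Spawninterval rate.
; Each tick, chained random rolls pick a rare ENEMYbig or ENEMYtime, otherwise the standard ENEMY.
; Spawn X and Y are random within hardcoded bounds, while Z comes from the Box component's height.
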(event Custom|spawn%20enemy
  (bind _returnvalue (Math|Random|RandomIntegerinRange 0 10))
  (if (== _returnvalue 0)
    (Game|SpawnActorfromClass "/Game/blueprint/enemy/ENEMY-big.ENEMY-big_C" (Math|Transform|MakeTransform (Math|Vector|MakeVector (Math|Random|RandomFloatinRange -2e+03 5e+03) (Math|Random|RandomFloatinRange -1.5e+03 4e+03) (.z (Transformation|GetWorldLocation (Variables|Default|GetBox)))) "0, 0, 0" "1.000000,1.000000,1.000000") "Undefined" "MultiplyWithRoot" 0 0)
    (elif (== _returnvalue 1)
      (Game|SpawnActorfromClass "/Game/blueprint/enemy/ENEMY-time.ENEMY-time_C" (Math|Transform|MakeTransform (Math|Vector|MakeVector (Math|Random|RandomFloatinRange -2e+03 5e+03) (Math|Random|RandomFloatinRange -1.5e+03 4e+03) (.z (Transformation|GetWorldLocation (Variables|Default|GetBox)))) "0, 0, 0" "1.000000,1.000000,1.000000") "Undefined" "MultiplyWithRoot" 0 0)
      (else
        (Game|SpawnActorfromClass "/Game/blueprint/enemy/ENEMY-.ENEMY-_C" (Math|Transform|MakeTransform (Math|Vector|MakeVector (Math|Random|RandomFloatinRange -2e+03 5e+03) (Math|Random|RandomFloatinRange -1.5e+03 4e+03) (.z (Transformation|GetWorldLocation (Variables|Default|GetBox)))) "0, 0, 0" "1.000000,1.000000,1.000000") "Undefined" "MultiplyWithRoot" 0 0)))))

(event EventBeginPlay
  (Utilities|Time|SetTimerbyFunctionName 0 "Spawn Enemy" (Variables|Default|Getspawninterval) true))

(fn ConstructionScript)